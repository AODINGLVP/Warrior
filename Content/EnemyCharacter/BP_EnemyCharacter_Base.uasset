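; Base enemy character Blueprint that handles the dissolve-based entrance and death effects.
; On BeginPlay, a reversed timeline drives DissolveAmount on the mesh while a random entry montage plays, then unhides the equipped weapon.
; On death, it freezes animation, disables capsule collision and clears widgets.
; It then async-loads a Niagara effect, tints it with the material's edge color, and dissolves the mesh before destroying weapon and actor.
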(event `self.ReceiveBeginPlay`
  (bind _entrymontagetoplay (`self.EntryMontageToPlay`))
  (bind _returnvalue (`PawnCombatComponent.GetCharacterCurrentEquippedWeapon` (`self.EnemyCombatComponent`)))
  (`|ExecutionSequence`
    (:`then_0`
      (`TimelineComponent.SetPlayRate` (`self.EntryRestoreTimeline`) (/ 1.0 (`self.TotalEntryRestorrTime`)))
      (bind (_direction _normalizedfloattrack) (`Timeline|EntryRestoreTimeline` :!via `ReverseFromEnd`)
        (:`Update`
          (`MeshComponent.SetScalarParameterValueOnMaterials` (`self.Mesh`) "DissolveAmount" _normalizedfloattrack))
        (:`Finished`
          (`/Engine/EditorBlueprintResources/StandardMacros.IsValid` _returnvalue
            (:`Is Valid`
              (`SceneComponent.SetHiddenInGame` (`WarriorWeaponBase.WeaponMesh` _returnvalue) false false))))))
    (:`then_1`
      (if (`KismetArrayLibrary.Array_IsNotEmpty` _entrymontagetoplay)
        (`self.PlayAnimMontage` (`KismetArrayLibrary.Array_Random` _entrymontagetoplay))))))

(event `/Game/EnemyCharacter/BP_EnemyDeath.OnEnemyDead`
  (params (DissolveNiagaraSystem :type "NiagaraSystem Soft Object Reference"))
  (bind _mesh (`self.Mesh`))
  (`|ExecutionSequence`
    (:`then_0`
      (set `SkeletalMeshComponent.bPauseAnims` true (`self.Mesh`))
      (`PrimitiveComponent.SetCollisionEnabled` (`self.CapsuleComponent`) "NoCollision"))
    (:`then_1`
      (`EnemyUIComponent.RemoveEnemyDrawnWidgetsIfAny` (`self.EnemyUIComponent`)))
    (:`then_2`
      (bind _object (`|LoadAsset` DissolveNiagaraSystem)
        (:`Completed`
          (bind _asniagara_system (cast `NiagaraSystem` _object))
          (bind _returnvalue (`NiagaraFunctionLibrary.SpawnSystemAttached` _asniagara_system (`self.Mesh`) "None" (0.0 0.0 0.0) (struct) "KeepRelativeOffset" true))
          (bind _returnvalue_2 (`PrimitiveComponent.CreateDynamicMaterialInstance` _mesh 0 (`PrimitiveComponent.GetMaterial` _mesh 0) "None"))
          (bind _returnvalue_3 (`MaterialInstanceDynamic.K2_GetVectorParameterValue` _returnvalue_2 "DissolveEdgeColor"))
          (`NiagaraComponent.SetNiagaraVariableLinearColor` _returnvalue "DissolveParticleColor" _returnvalue_3)
          (`TimelineComponent.SetPlayRate` (`self.Timeline`) (/ 1.0 (`self.TotalDissolveTime`)))
          (bind (_direction _normalizedfloattrack) (`Timeline|Timeline` :!via `PlayFromStart`)
            (:`Update`
              (`MeshComponent.SetScalarParameterValueOnMaterials` (`self.Mesh`) "DissolveAmount" _normalizedfloattrack))
            (:`Finished`
              (`self.K2_DestroyActor` (`PawnCombatComponent.GetCharacterCurrentEquippedWeapon` (`self.EnemyCombatComponent`)))
              (`self.K2_DestroyActor`))))))))

(fn `UserConstructionScript`)