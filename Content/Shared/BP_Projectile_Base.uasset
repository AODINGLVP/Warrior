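; Base projectile Blueprint that provides the sound and visual effects for projectile spawn, flight and impact.
; On BeginPlay it plays a spawn sound, attaches a flight sound that stops with the projectile, and spawns a forward-facing muzzle effect.
; The OnSpawnProjectileHitFX event plays the impact sound and effect at a supplied hit location.
; Each asset is validity-checked before use, and this graph contains no movement, collision or damage logic.
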(event `self.ReceiveBeginPlay`
  (`|ExecutionSequence`
    (:`then_0`
      (bind _projectilespawnsound (`self.projectilespawnsound`)
        (:`then`
          (`GameplayStatics.PlaySoundAtLocation` _projectilespawnsound (`self.K2_GetActorLocation`) (struct) 1.0 1.0 0.0 null null null null))
        (:`else`)))
    (:`then_1`
      (bind _projectflysound (`self.projectflysound`)
        (:`then`
          (`GameplayStatics.SpawnSoundAttached` _projectflysound (`self.RootComponent`) "None" (0.0 0.0 0.0) (struct) "KeepRelativeOffset" true 1.0 1.0 0.0 null null))
        (:`else`)))
    (:`then_2`
      (bind _projectmuzziefx (`self.projectmuzziefx`)
        (:`then`
          (`NiagaraFunctionLibrary.SpawnSystemAtLocation` _projectmuzziefx (`self.K2_GetActorLocation`) (`KismetMathLibrary.Conv_VectorToRotator` (`self.GetActorForwardVector`))))
        (:`else`)))))

(event `self.BP_OnSpawnProjectileHitFX`
  (params (HitLocation :type "Vector Structure (by ref)"))
  (`|ExecutionSequence`
    (:`then_0`
      (bind _sound (`self.Sound`)
        (:`then`
          (`GameplayStatics.PlaySoundAtLocation` _sound HitLocation (struct) 1.0 1.0 0.0 null null null null))
        (:`else`)))
    (:`then_1`
      (bind _projectileimpactfx (`self.ProjectileImpactFX`)
        (:`then`
          (`NiagaraFunctionLibrary.SpawnSystemAtLocation` _projectileimpactfx HitLocation))
        (:`else`)))))

(fn `UserConstructionScript`)